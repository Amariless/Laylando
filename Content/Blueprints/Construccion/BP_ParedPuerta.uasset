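; Wall-with-door actor whose door swings open when an actor overlaps it and closes when an overlap ends.
; Overlap events toggle the AbriendoPuerta flag without filtering the other actor, and print a debug message.
; Tick reads the flag and uses RInterpTo to ease SMPuerta2's relative rotation toward the open or closed angle, opening faster than it closes.
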(event `self.ReceiveTick`
  (params (DeltaSeconds :type "Float (single-precision)"))
  (bind _sm_puerta2 (`self.SM_Puerta2`))
  (bind _sm_puerta2_2 (`self.SM_Puerta2`))
  (if (`self.AbriendoPuerta`)
    (`SceneComponent.K2_SetRelativeRotation` _sm_puerta2_2 (`KismetMathLibrary.RInterpTo` (`SceneComponent.RelativeRotation` _sm_puerta2_2) (struct :`Yaw` 100.0) DeltaSeconds 2.0) false false)
    (else
      (`SceneComponent.K2_SetRelativeRotation` _sm_puerta2 (`KismetMathLibrary.RInterpTo` (`SceneComponent.RelativeRotation` _sm_puerta2) (struct) DeltaSeconds 1.0) false false))))

(event `self.ReceiveActorBeginOverlap`
  (params (OtherActor :type "Actor Object Reference"))
  (set `self.AbriendoPuerta` true)
  (`KismetSystemLibrary.PrintText` "Abriendo puerta" true true (struct :`G` 0.252201 :`B` 1.0 :`A` 1.0) 3.0))

(event `self.ReceiveActorEndOverlap`
  (params (OtherActor :type "Actor Object Reference"))
  (set `self.AbriendoPuerta` false)
  (`KismetSystemLibrary.PrintText` "Cerrando puerta" true true (struct :`G` 0.252201 :`B` 1.0 :`A` 1.0) 3.0))

(event `self.ReceiveBeginPlay`
  (set `self.AbriendoPuerta` false))

(fn `UserConstructionScript`)